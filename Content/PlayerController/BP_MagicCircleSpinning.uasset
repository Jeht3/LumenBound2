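; Magic circle actor that continuously spins and rescales its Ring component.
; On BeginPlay, the SpinningRing timeline drives the ring's yaw and Z scale, then restarts itself after a tiny delay each time it finishes.
; The WinBox overlap event is empty; disconnected leftover logic for a player win screen, with sound and game pause, never runs.
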(event `self.ReceiveBeginPlay`
  (bind _ring (`self.Ring`))
  (bind _ring_2 (`self.Ring`))
  (bind (_relativerotation_roll _relativerotation_pitch) (`KismetMathLibrary.BreakRotator` (`SceneComponent.RelativeRotation` _ring_2)))
  (bind (_relativescale3d_x _relativescale3d_y) (`KismetMathLibrary.BreakVector` (`SceneComponent.RelativeScale3D` _ring)))
  (`/Engine/EditorBlueprintResources/StandardMacros.DoOnce` false
    (:`Completed`
      (bind (_direction _rotation _scale) (`Timeline|SpinningRing` :!via `PlayFromStart` :!label _label)
        (:`Update`
          (`|ExecutionSequence`
            (:`then_0`
              (`SceneComponent.K2_SetRelativeRotation` _ring_2 (`KismetMathLibrary.MakeRotator` _relativerotation_roll _relativerotation_pitch _rotation) false false))
            (:`then_1`
              (`SceneComponent.SetRelativeScale3D` _ring (`KismetMathLibrary.MakeVector` _relativescale3d_x _relativescale3d_y _scale)))))
        (:`Finished`
          (`KismetSystemLibrary.Delay` 0.001)
          (goto _label :!via `PlayFromStart`))))))

(event `self.WinBox.OnComponentBeginOverlap`
  (params (OverlappedComponent :type "PrimitiveComponent Object Reference") (OtherActor :type "Actor Object Reference") (OtherComp :type "PrimitiveComponent Object Reference") (OtherBodyIndex :type Integer) (bFromSweep :type Boolean) (SweepResult :type "HitResult Structure (by ref)")))

(fn `UserConstructionScript`)