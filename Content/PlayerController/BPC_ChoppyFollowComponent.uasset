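; BPC_ChoppyFollowComponent is an actor component that makes its owner follow a target in discrete, choppy steps.
; On BeginPlay it starts a looping timer at UpdateInterval that calls UpdateChoppyTransform.
; Each tick of that timer snaps the owner's root component to the world location and rotation of TargetComponent's root, with no sweep or interpolation.
; TargetComponent is used as an actor reference despite its name, and is not null-checked.
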(event `self.ReceiveBeginPlay`
  (`KismetSystemLibrary.K2_SetTimer` null "UpdateChoppyTransform" (`self.UpdateInterval`) true))

(event `UpdateChoppyTransform`
  (bind _rootcomponent (`Actor.RootComponent` (`self.GetOwner`)))
  (bind _rootcomponent_2 (`Actor.RootComponent` (`self.TargetComponent`)))
  (`SceneComponent.K2_SetWorldLocation` _rootcomponent (`SceneComponent.K2_GetComponentLocation` _rootcomponent_2) false false)
  (`SceneComponent.K2_SetWorldRotation` _rootcomponent (`SceneComponent.K2_GetComponentRotation` _rootcomponent_2) false false))