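; BP_Door is a double door that opens once the player has enough skeleton and lamp charges.
; On BeginPlay it caches the BP_Player and reveals up to three skeleton and lantern markers to match NeededCharges.
; Tick polls both of the player's charge counts against NeededCharges and fires OpenDoors through a DoOnce.
; OpenDoors swings both leaves apart in delayed, stepped rotations, playing a sound at each step.
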(event `self.ReceiveBeginPlay`
  (bind _asbp_player (cast `/Game/PlayerController/BP_Player` (`GameplayStatics.GetPlayerPawn` 0)))
  (set `self.PlayerRef` _asbp_player)
  (if (>= (`self.NeededCharges`) 1.0)
    (`SceneComponent.SetVisibility` (`self.1Skele`) true false)
    (`SceneComponent.SetVisibility` (`self.1Lantern`) true false)
    (if (>= (`self.NeededCharges`) 2.0)
      (`SceneComponent.SetVisibility` (`self.2Skele`) true false)
      (`SceneComponent.SetVisibility` (`self.2Lantern`) true false)
      (if (>= (`self.NeededCharges`) 3.0)
        (`SceneComponent.SetVisibility` (`self.3Skele`) true false)
        (`SceneComponent.SetVisibility` (`self.3Lantern`) true false)))))

(event `self.ReceiveTick`
  (params (DeltaSeconds :type "Float (single-precision)"))
  (if (and (>= (`/Game/PlayerController/BP_Player.SkeletonCharges` (`self.PlayerRef`)) (`self.NeededCharges`)) (>= (`/Game/PlayerController/BP_Player.LampCharges` (`self.PlayerRef`)) (`self.NeededCharges`)))
    (`/Engine/EditorBlueprintResources/StandardMacros.DoOnce` false
      (:`Completed`
        (`self.OpenDoors`)))))

(event `OpenDoors`
  (`KismetSystemLibrary.Delay` 1.0)
  (`GameplayStatics.PlaySound2D` "/Game/PlayerController/Sounds/Doors.Doors" 1.0 1.0 0.0 null null)
  (`SceneComponent.K2_SetRelativeRotation` (`self.Door`) (struct :`Yaw` -30.0) false false)
  (`SceneComponent.K2_SetRelativeRotation` (`self.Door2`) (struct :`Yaw` 30.0) false false)
  (`KismetSystemLibrary.Delay` 0.5)
  (`GameplayStatics.PlaySound2D` "/Game/PlayerController/Sounds/Doors.Doors" 1.0 1.0 0.0 null null)
  (`SceneComponent.K2_SetRelativeRotation` (`self.Door`) (struct :`Yaw` -60.0) false false)
  (`SceneComponent.K2_SetRelativeRotation` (`self.Door2`) (struct :`Yaw` 60.0) false false)
  (`KismetSystemLibrary.Delay` 0.5)
  (`GameplayStatics.PlaySound2D` "/Game/PlayerController/Sounds/Doors.Doors" 1.0 1.0 0.0 null null)
  (`SceneComponent.K2_SetRelativeRotation` (`self.Door`) (struct :`Yaw` -90.0) false false)
  (`SceneComponent.K2_SetRelativeRotation` (`self.Door2`) (struct :`Yaw` 90.0) false false))

(fn `UserConstructionScript`)