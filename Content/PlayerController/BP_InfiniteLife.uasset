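; BP_InfiniteLife tops up the player's life and lantern light for as long as its GiveValue flag is on.
; On BeginPlay it caches the first player pawn as a BP_Player reference.
; Each Tick with the flag set adds a fixed amount to LifeValue and LanternLightValue, with no delta-time scaling or clamping.
; Nothing in these graphs sets the flag.
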(event `self.ReceiveBeginPlay`
  (bind _asbp_player (cast `/Game/PlayerController/BP_Player` (`GameplayStatics.GetPlayerPawn` 0)))
  (set `self.PlayerRef` _asbp_player))

(event `self.ReceiveTick`
  (params (DeltaSeconds :type "Float (single-precision)"))
  (bind _playerref (`self.PlayerRef`))
  (if (`self.GiveValue?`)
    (set `/Game/PlayerController/BP_Player.LanternLightValue` (+ (`/Game/PlayerController/BP_Player.LanternLightValue` _playerref) 4.0) _playerref)
    (set `/Game/PlayerController/BP_Player.LifeValue` (+ (`/Game/PlayerController/BP_Player.LifeValue` _playerref) 4.0) _playerref)))

(fn `UserConstructionScript`)