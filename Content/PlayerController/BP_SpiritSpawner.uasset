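; BP_SpiritSpawner is a spawner actor that continuously creates BP_Spirit actors within a box volume.
; On BeginPlay a looping timer fires every fraction of a second, spawning a spirit at a random X/Y inside the trigger box, at the box center's height.
; Player overlap events only cast to BP_Player, and the timer-clearing stop event is never called here, so spawning runs regardless of player presence.
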(event `StopSpawningActors`
  (`KismetSystemLibrary.K2_ClearAndInvalidateTimerHandle` (stale `self.ReceiveBeginPlay` _returnvalue)))

(event `self.SpawnActors_Trigger.OnComponentBeginOverlap`
  (params (OverlappedComponent :type "PrimitiveComponent Object Reference") (OtherActor :type "Actor Object Reference") (OtherComp :type "PrimitiveComponent Object Reference") (OtherBodyIndex :type Integer) (bFromSweep :type Boolean) (SweepResult :type "HitResult Structure (by ref)"))
  (cast `/Game/PlayerController/BP_Player` OtherActor))

(event `self.ReceiveBeginPlay`
  (bind _returnvalue (`KismetSystemLibrary.K2_SetTimerDelegate` (delegate `SpawnActorsOvertime`) 0.6 true)))

(event `SpawnActorsOvertime`
  (bind _spawnactors_trigger (`self.SpawnActors_Trigger`))
  (bind _returnvalue (`SceneComponent.K2_GetComponentLocation` _spawnactors_trigger))
  (bind (_returnvalue_x _returnvalue_y) (`KismetMathLibrary.BreakVector` (`KismetMathLibrary.RandomPointInBoundingBox` _returnvalue (`BoxComponent.BoxExtent` _spawnactors_trigger))))
  (`|SpawnActorFromClass` "/Game/PlayerController/BP_Spirit.BP_Spirit_C" (`KismetMathLibrary.MakeTransform` (`KismetMathLibrary.MakeVector` _returnvalue_x _returnvalue_y (.z _returnvalue))) "Undefined" "MultiplyWithRoot" null null))

(event `self.SpawnActors_Trigger.OnComponentEndOverlap`
  (params (OverlappedComponent :type "PrimitiveComponent Object Reference") (OtherActor :type "Actor Object Reference") (OtherComp :type "PrimitiveComponent Object Reference") (OtherBodyIndex :type Integer))
  (cast `/Game/PlayerController/BP_Player` OtherActor))

(fn `UserConstructionScript`)