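; BP_LanternCharge is a pickup that grants the player a lantern charge.
; A looping timer spins the Spirit component in steps and randomly nudges its height, also adding its current relative X and Y as deltas.
; DestroyCharge runs once, calling LanternChargeGet on BP_Player, hiding Spirit and NSSpiritEnergy, and playing a pickup sound.
; The actor is hidden rather than destroyed, and its own overlap event is unused.
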(event `self.ReceiveBeginPlay`
  (`KismetSystemLibrary.K2_SetTimerDelegate` (delegate `Spin`) 0.3 true))

(event `Spin`
  (bind _spirit (`self.Spirit`))
  (bind (_relativelocation_x _relativelocation_y) (`KismetMathLibrary.BreakVector` (`SceneComponent.RelativeLocation` _spirit)))
  (`SceneComponent.K2_AddRelativeRotation` _spirit (struct :`Yaw` 30.0) false false)
  (`SceneComponent.K2_AddRelativeLocation` _spirit (`KismetMathLibrary.MakeVector` _relativelocation_x _relativelocation_y (`KismetMathLibrary.RandomFloatInRange` -5.0 5.0)) false false))

(event `DestroyCharge`
  (`/Engine/EditorBlueprintResources/StandardMacros.DoOnce` false
    (:`Completed`
      (bind _asbp_player (cast `/Game/PlayerController/BP_Player` (`GameplayStatics.GetPlayerPawn` 0)))
      (`/Game/PlayerController/BP_Player.LanternChargeGet` _asbp_player)
      (`SceneComponent.SetVisibility` (`self.Spirit`) false false)
      (`SceneComponent.SetVisibility` (`self.NS_SpiritEnergy`) false false)
      (`GameplayStatics.PlaySound2D` "/Game/PlayerController/Sounds/pickupCoin__2_.pickupCoin__2_" 1.0 1.0 0.0 null null))))

(fn `UserConstructionScript`)