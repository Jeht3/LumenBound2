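; BP_ObjectGrow tracks a grow charge value and shows or hides its Widget component to match.
; Each Tick raises ObjectGrowValue while IsCharging is set and lowers it otherwise, clamped between zero and a maximum, in fixed steps not scaled by delta time.
; The widget appears once charge builds and hides when it drains below zero.
; Nothing here sets IsCharging or applies the value to an object.
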(event `self.ReceiveTick`
  (params (DeltaSeconds :type "Float (single-precision)"))
  (if (`self.IsCharging?`)
    (`|ExecutionSequence`
      (:`then_0`
        (bind _output_get (set `self.ObjectGrowValue` (+ (`self.ObjectGrowValue`) 5.0)))
        (if (> (`self.ObjectGrowValue`) 1000.0)
          (set `self.ObjectGrowValue` 1000.0)))
      (:`then_1`
        (if (> (`self.ObjectGrowValue`) 1.0)
          (`SceneComponent.SetVisibility` (`self.Widget`) true false))))
    (else
      (bind _output_get_2 (set `self.ObjectGrowValue` (- (`self.ObjectGrowValue`) 5.0)))
      (if (< (`self.ObjectGrowValue`) 0.0)
        (set `self.ObjectGrowValue` 0.0)
        (`SceneComponent.SetVisibility` (`self.Widget`) false false)))))

(fn `UserConstructionScript`)