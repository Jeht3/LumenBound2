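; BP_Arrow is a direction indicator actor that follows the player pawn and turns relative to a fixed, hard-coded world location.
; Every tick it moves Arrow1 to the pawn's location, then calls RotateArrow.
; RotateArrow sets only the relative yaw, derived from the vector between that point and the player plus a 90-degree offset, keeping roll and pitch unchanged.
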(event `self.ReceiveBeginPlay`
  (set `self.PlayerRef` (`GameplayStatics.GetPlayerPawn` 0)))

(event `self.ReceiveTick`
  (params (DeltaSeconds :type "Float (single-precision)"))
  (`|ExecutionSequence`
    (:`then_0`
      (`SceneComponent.K2_SetWorldLocation` (`self.Arrow1`) (`self.K2_GetActorLocation` (`self.PlayerRef`)) false false))
    (:`then_1`
      (`self.RotateArrow`))))

(event `RotateArrow`
  (bind _arrow1 (`self.Arrow1`))
  (bind (_relativerotation_roll _relativerotation_pitch) (`KismetMathLibrary.BreakRotator` (`SceneComponent.RelativeRotation` _arrow1)))
  (bind (_returnvalue_roll _returnvalue_pitch _returnvalue_yaw) (`KismetMathLibrary.BreakRotator` (`KismetMathLibrary.MakeRotFromX` (- (`self.K2_GetActorLocation` (`self.PlayerRef`)) (2630.0 3080.0 45.0)))))
  (`SceneComponent.K2_SetRelativeRotation` _arrow1 (`KismetMathLibrary.MakeRotator` _relativerotation_roll _relativerotation_pitch (+ _returnvalue_yaw 90.0)) false false))

(fn `UserConstructionScript`)