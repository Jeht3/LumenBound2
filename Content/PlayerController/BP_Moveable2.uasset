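; BP_Moveable2 moves a referenced object through preset transforms as its linked charger fills and empties.
; Tick polls the charger's ObjectGrowValue, playing three stepped location, rotation and scale changes above 999.
; Below 1, it steps back through them to the starting transform.
; Two DoOnce gates, the uncharge one starting closed, re-arm each other after each delayed sequence so the directions alternate.
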(event `self.ReceiveTick`
  (params (DeltaSeconds :type "Float (single-precision)"))
  (`|ExecutionSequence`
    (:`then_0`
      (if (> (`/Game/PlayerController/BP_Lever.ObjectGrowValue` (`self.ChargerRef`)) 999.0)
        (`/Engine/EditorBlueprintResources/StandardMacros.DoOnce` false :!label _label
          (:`Completed`
            (`self.IsDoneCharging`)))))
    (:`then_1`
      (if (< (`/Game/PlayerController/BP_Lever.ObjectGrowValue` (`self.ChargerRef`)) 1.0)
        (`/Engine/EditorBlueprintResources/StandardMacros.DoOnce` true :!label _label_2
          (:`Completed`
            (`self.UnCharge`)))))))

(event `IsDoneCharging`
  (bind _rootcomponent (`Actor.RootComponent` (`self.ObjectRef`)))
  (bind _rootcomponent_2 (`Actor.RootComponent` (`self.ObjectRef`)))
  (bind _rootcomponent_3 (`Actor.RootComponent` (`self.ObjectRef`)))
  (`SceneComponent.K2_SetWorldLocationAndRotation` _rootcomponent (`self.Location1`) (`self.Rotation1`) false false)
  (`SceneComponent.SetWorldScale3D` _rootcomponent (`self.Scale1`))
  (`KismetSystemLibrary.Delay` 0.5)
  (`SceneComponent.K2_SetWorldLocationAndRotation` _rootcomponent_2 (`self.Location2`) (`self.Rotation2`) false false)
  (`SceneComponent.SetWorldScale3D` _rootcomponent_2 (`self.Scale2`))
  (`KismetSystemLibrary.Delay` 0.5)
  (`SceneComponent.K2_SetWorldLocationAndRotation` _rootcomponent_3 (`self.Location3`) (`self.Rotation3`) false false)
  (`SceneComponent.SetWorldScale3D` _rootcomponent_3 (`self.Scale3`))
  (goto _label_2 :!via `Reset`))

(event `UnCharge`
  (bind _rootcomponent (`Actor.RootComponent` (`self.ObjectRef`)))
  (bind _rootcomponent_2 (`Actor.RootComponent` (`self.ObjectRef`)))
  (bind _rootcomponent_3 (`Actor.RootComponent` (`self.ObjectRef`)))
  (`SceneComponent.K2_SetWorldLocationAndRotation` _rootcomponent (`self.Location2`) (`self.Rotation2`) false false)
  (`SceneComponent.SetWorldScale3D` _rootcomponent (`self.Scale2`))
  (`KismetSystemLibrary.Delay` 0.5)
  (`SceneComponent.K2_SetWorldLocationAndRotation` _rootcomponent_3 (`self.Location1`) (`self.Rotation1`) false false)
  (`SceneComponent.SetWorldScale3D` _rootcomponent_3 (`self.Scale1`))
  (`KismetSystemLibrary.Delay` 0.5)
  (`SceneComponent.K2_SetWorldLocationAndRotation` _rootcomponent_2 (`self.StartingLocation`) (`self.StartingRotation`) false false)
  (`SceneComponent.SetWorldScale3D` _rootcomponent_2 (`self.StartingScale`))
  (goto _label :!via `Reset`))

(fn `UserConstructionScript`)