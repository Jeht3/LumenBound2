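; BP_Spirit is a spirit actor with a Cube component that grows in on spawn and drifts in a random direction.
; BeginPlay picks two random offsets and plays the SpawningIn timeline, which drives the Cube's uniform relative scale.
; Tick adds those fixed offsets to the Cube's relative X and Y every frame, without delta-time scaling, so drift speed depends on frame rate.
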(event `self.ReceiveBeginPlay`
  (set `self.RandomFloat1` (`KismetMathLibrary.RandomFloatInRange` -3.0 3.0))
  (set `self.RandomFloat2` (`KismetMathLibrary.RandomFloatInRange` -3.0 3.0))
  (bind (_direction _scale) (`Timeline|SpawningIn` :!via `PlayFromStart`)
    (:`Update`
      (`SceneComponent.SetRelativeScale3D` (`self.Cube`) (`KismetMathLibrary.Conv_DoubleToVector` _scale)))))

(event `self.ReceiveTick`
  (params (DeltaSeconds :type "Float (single-precision)"))
  (`SceneComponent.K2_AddRelativeLocation` (`self.Cube`) (`KismetMathLibrary.MakeVector` (`self.RandomFloat1`) (`self.RandomFloat2`)) false false))

(fn `UserConstructionScript`)