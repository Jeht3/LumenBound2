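; BP_SkeletonCharge is a pickup actor that grants the player a skeleton charge.
; A looping timer rotates the Spirit component in steps and nudges it by a random vertical offset, feeding its current relative X and Y back as deltas.
; When BP_Player overlaps the Sphere, a DoOnce gate calls SkeletonChargeGet on that player, plays a pickup sound and destroys the actor.
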(event `self.ReceiveBeginPlay`
  (`KismetSystemLibrary.K2_SetTimerDelegate` (delegate `Spin`) 0.3 true))

(event `Spin`
  (bind _spirit (`self.Spirit`))
  (bind (_relativelocation_x _relativelocation_y) (`KismetMathLibrary.BreakVector` (`SceneComponent.RelativeLocation` _spirit)))
  (`SceneComponent.K2_AddRelativeRotation` _spirit (struct :`Yaw` 30.0) false false)
  (`SceneComponent.K2_AddRelativeLocation` _spirit (`KismetMathLibrary.MakeVector` _relativelocation_x _relativelocation_y (`KismetMathLibrary.RandomFloatInRange` -5.0 5.0)) false false))

(event `self.Sphere.OnComponentBeginOverlap`
  (params (OverlappedComponent :type "PrimitiveComponent Object Reference") (OtherActor :type "Actor Object Reference") (OtherComp :type "PrimitiveComponent Object Reference") (OtherBodyIndex :type Integer) (bFromSweep :type Boolean) (SweepResult :type "HitResult Structure (by ref)"))
  (bind _asbp_player (cast `/Game/PlayerController/BP_Player` OtherActor))
  (`/Engine/EditorBlueprintResources/StandardMacros.DoOnce` false
    (:`Completed`
      (`/Game/PlayerController/BP_Player.SkeletonChargeGet` _asbp_player)
      (`GameplayStatics.PlaySound2D` "/Game/PlayerController/Sounds/pickupCoin__2_.pickupCoin__2_" 1.0 1.0 0.0 null null)
      (`self.K2_DestroyActor`))))

(fn `UserConstructionScript`)