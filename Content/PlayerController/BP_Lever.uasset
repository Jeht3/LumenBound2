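; BP_Lever is a one-shot lever that throws itself when BP_Player overlaps its capsule.
; MoveLever steps the handle through five fixed rotations using timed delays, playing a sound at each step, then sets ObjectGrowValue to its full value.
; Tick is empty, and leftover charge/decay logic that would ramp ObjectGrowValue and toggle a widget is disconnected.
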(event `self.ReceiveTick`
  (params (DeltaSeconds :type "Float (single-precision)")))

(event `self.Capsule.OnComponentBeginOverlap`
  (params (OverlappedComponent :type "PrimitiveComponent Object Reference") (OtherActor :type "Actor Object Reference") (OtherComp :type "PrimitiveComponent Object Reference") (OtherBodyIndex :type Integer) (bFromSweep :type Boolean) (SweepResult :type "HitResult Structure (by ref)"))
  (cast `/Game/PlayerController/BP_Player` OtherActor)
  (`/Engine/EditorBlueprintResources/StandardMacros.DoOnce` false
    (:`Completed`
      (`self.MoveLever`))))

(event `MoveLever`
  (`KismetSystemLibrary.Delay` 0.5)
  (`GameplayStatics.PlaySound2D` "/Game/PlayerController/Sounds/lever.lever" 1.0 1.0 0.0 null null)
  (`SceneComponent.K2_SetRelativeRotation` (`self.LeverHandle`) (struct :`Pitch` -50.0) false false)
  (`KismetSystemLibrary.Delay` 0.5)
  (`GameplayStatics.PlaySound2D` "/Game/PlayerController/Sounds/lever.lever" 1.0 1.0 0.0 null null)
  (`SceneComponent.K2_SetRelativeRotation` (`self.LeverHandle`) (struct :`Pitch` -25.0) false false)
  (`KismetSystemLibrary.Delay` 0.5)
  (`GameplayStatics.PlaySound2D` "/Game/PlayerController/Sounds/lever.lever" 1.0 1.0 0.0 null null)
  (`SceneComponent.K2_SetRelativeRotation` (`self.LeverHandle`) (struct) false false)
  (`KismetSystemLibrary.Delay` 0.5)
  (`GameplayStatics.PlaySound2D` "/Game/PlayerController/Sounds/lever.lever" 1.0 1.0 0.0 null null)
  (`SceneComponent.K2_SetRelativeRotation` (`self.LeverHandle`) (struct :`Pitch` 25.0) false false)
  (`KismetSystemLibrary.Delay` 0.5)
  (`GameplayStatics.PlaySound2D` "/Game/PlayerController/Sounds/lever.lever" 1.0 1.0 0.0 null null)
  (`SceneComponent.K2_SetRelativeRotation` (`self.LeverHandle`) (struct :`Pitch` 50.0) false false)
  (`KismetSystemLibrary.Delay` 0.5)
  (set `self.ObjectGrowValue` 1000.0))

(fn `UserConstructionScript`)