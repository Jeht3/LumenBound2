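; BP_Moveable steps a referenced static mesh between preset transforms as a charger's grow value reaches its extremes.
; Tick polls ChargerRef, firing IsDoneCharging near full charge and UnCharge near empty, each behind a DoOnce.
; Both events snap location, rotation and scale through three stages with half-second delays, forward when charged and back to the starting transform when drained.
; Each sequence re-arms the opposite DoOnce when it finishes.
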(event `self.ReceiveTick`
  (params (DeltaSeconds :type "Float (single-precision)"))
  (`|ExecutionSequence`
    (:`then_0`
      (if (> (`/Game/PlayerController/BP_ObjectGrow.ObjectGrowValue` (`self.ChargerRef`)) 999.0)
        (`/Engine/EditorBlueprintResources/StandardMacros.DoOnce` false :!label _label
          (:`Completed`
            (`self.IsDoneCharging`)))))
    (:`then_1`
      (if (< (`/Game/PlayerController/BP_ObjectGrow.ObjectGrowValue` (`self.ChargerRef`)) 1.0)
        (`/Engine/EditorBlueprintResources/StandardMacros.DoOnce` false :!label _label_2
          (:`Completed`
            (`self.UnCharge`)))))))

(event `IsDoneCharging`
  (bind _staticmeshcomponent (`StaticMeshActor.StaticMeshComponent` (`self.ObjectRef`)))
  (bind _staticmeshcomponent_2 (`StaticMeshActor.StaticMeshComponent` (`self.ObjectRef`)))
  (bind _staticmeshcomponent_3 (`StaticMeshActor.StaticMeshComponent` (`self.ObjectRef`)))
  (`SceneComponent.K2_SetWorldLocationAndRotation` _staticmeshcomponent (`self.Location1`) (`self.Rotation1`) false false)
  (`SceneComponent.SetWorldScale3D` _staticmeshcomponent (`self.Scale1`))
  (`KismetSystemLibrary.Delay` 0.5)
  (`SceneComponent.K2_SetWorldLocationAndRotation` _staticmeshcomponent_2 (`self.Location2`) (`self.Rotation2`) false false)
  (`SceneComponent.SetWorldScale3D` _staticmeshcomponent_2 (`self.Scale2`))
  (`KismetSystemLibrary.Delay` 0.5)
  (`SceneComponent.K2_SetWorldLocationAndRotation` _staticmeshcomponent_3 (`self.Location3`) (`self.Rotation3`) false false)
  (`SceneComponent.SetWorldScale3D` _staticmeshcomponent_3 (`self.Scale3`))
  (goto _label_2 :!via `Reset`))

(event `UnCharge`
  (bind _staticmeshcomponent (`StaticMeshActor.StaticMeshComponent` (`self.ObjectRef`)))
  (bind _staticmeshcomponent_2 (`StaticMeshActor.StaticMeshComponent` (`self.ObjectRef`)))
  (bind _staticmeshcomponent_3 (`StaticMeshActor.StaticMeshComponent` (`self.ObjectRef`)))
  (`SceneComponent.K2_SetWorldLocationAndRotation` _staticmeshcomponent (`self.Location2`) (`self.Rotation2`) false false)
  (`SceneComponent.SetWorldScale3D` _staticmeshcomponent (`self.Scale2`))
  (`KismetSystemLibrary.Delay` 0.5)
  (`SceneComponent.K2_SetWorldLocationAndRotation` _staticmeshcomponent_2 (`self.Location1`) (`self.Rotation1`) false false)
  (`SceneComponent.SetWorldScale3D` _staticmeshcomponent_2 (`self.Scale1`))
  (`KismetSystemLibrary.Delay` 0.5)
  (`SceneComponent.K2_SetWorldLocationAndRotation` _staticmeshcomponent_3 (`self.StartingLocation`) (`self.StartingRotation`) false false)
  (`SceneComponent.SetWorldScale3D` _staticmeshcomponent_3 (`self.StartingScale`))
  (goto _label :!via `Reset`))

(fn `UserConstructionScript`)