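; BP_Lightsource is a light source that refills the player's lantern while the player stands inside its Box trigger.
; BeginPlay caches player 0's BP_Player pawn, and the box's begin and end overlap events toggle a GiveValue flag for that class.
; While the flag is set, Tick adds a fixed amount to LanternLightValue with no delta-time scaling or clamp here.
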(event `self.ReceiveBeginPlay`
  (bind _asbp_player (cast `/Game/PlayerController/BP_Player` (`GameplayStatics.GetPlayerPawn` 0)))
  (set `self.PlayerRef` _asbp_player))

(event `self.ReceiveTick`
  (params (DeltaSeconds :type "Float (single-precision)"))
  (bind _playerref (`self.PlayerRef`))
  (if (`self.GiveValue?`)
    (set `/Game/PlayerController/BP_Player.LanternLightValue` (+ (`/Game/PlayerController/BP_Player.LanternLightValue` _playerref) 4.0) _playerref)))

(event `self.Box.OnComponentBeginOverlap`
  (params (OverlappedComponent :type "PrimitiveComponent Object Reference") (OtherActor :type "Actor Object Reference") (OtherComp :type "PrimitiveComponent Object Reference") (OtherBodyIndex :type Integer) (bFromSweep :type Boolean) (SweepResult :type "HitResult Structure (by ref)"))
  (cast `/Game/PlayerController/BP_Player` OtherActor)
  (set `self.GiveValue?` true))

(event `self.Box.OnComponentEndOverlap`
  (params (OverlappedComponent :type "PrimitiveComponent Object Reference") (OtherActor :type "Actor Object Reference") (OtherComp :type "PrimitiveComponent Object Reference") (OtherBodyIndex :type Integer))
  (cast `/Game/PlayerController/BP_Player` OtherActor)
  (set `self.GiveValue?` false))

(fn `UserConstructionScript`)